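; BP_PhysicsPickup is an interactable physics cube that the player can pick up and drop.
; On interact, if the player holds nothing, it sets the player's holding flag, disables cube physics and collision, and attaches the cube to the player's camera.
; The drop event detaches the actor and restores collision and physics, leaving the holding flag untouched.
; The construction script tints the cube with PickupColor through a dynamic material.
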(event `/Game/Charlie_EnemyAI_Sandbox/AnimatedInteractables/Interface_Interact.INT_Interact`
  (params (BP_PlayerChar :type "/Game/Charlie_EnemyAI_Sandbox/Player/BP_PlayerChar Object Reference"))
  (bind _cube (`self.Cube`))
  (if (not (`/Game/Charlie_EnemyAI_Sandbox/Player/BP_PlayerChar.isholding?` BP_PlayerChar))
    (set `/Game/Charlie_EnemyAI_Sandbox/Player/BP_PlayerChar.isholding?` true BP_PlayerChar)
    (`PrimitiveComponent.SetSimulatePhysics` _cube false)
    (`PrimitiveComponent.SetCollisionEnabled` _cube "NoCollision")
    (`SceneComponent.K2_AttachToComponent` (`self.Cube`) (`/Game/Charlie_EnemyAI_Sandbox/Player/BP_PlayerChar.Camera1` BP_PlayerChar) "None" "KeepWorld" "KeepWorld" "KeepWorld" true)))

(event `/Game/Charlie_EnemyAI_Sandbox/AnimatedInteractables/Interface_Interact.INT_Drop`
  (params (`BP_Player Char` :type "/Game/Charlie_EnemyAI_Sandbox/Player/BP_PlayerChar Object Reference"))
  (bind _cube (`self.Cube`))
  (`self.K2_DetachFromActor` "KeepWorld" "KeepWorld" "KeepWorld")
  (`PrimitiveComponent.SetCollisionEnabled` _cube "QueryAndPhysics")
  (`PrimitiveComponent.SetSimulatePhysics` _cube true))

(fn `UserConstructionScript`
  (bind _returnvalue (`PrimitiveComponent.CreateDynamicMaterialInstance` (`self.Cube`) 0 "/Game/Charlie_EnemyAI_Sandbox/AnimatedInteractables/MAT_Color.MAT_Color" "None"))
  (bind _output_get (set `self.ColorDMI` _returnvalue))
  (`MaterialInstanceDynamic.SetVectorParameterValue` _output_get "Color" (`self.PickupColor`)))