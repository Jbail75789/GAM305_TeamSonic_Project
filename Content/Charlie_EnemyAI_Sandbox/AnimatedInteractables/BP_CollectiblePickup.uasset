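; BP_CollectiblePickup is a spinning cube pickup that boosts the player's health when interacted with.
; Tick rotates the cube, and the INTInteract interface event casts the target to BP_PlayerChar.
; It sets both max health and current health to a fixed value, refreshes the health widget, then destroys itself.
; A Float timeline meant to move the cube vertically is present but never runs.
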(event `self.ReceiveTick`
  (params (DeltaSeconds :type "Float (single-precision)"))
  (`SceneComponent.K2_AddWorldRotation` (`self.Cube`) (struct :`Yaw` 2.0) false false))

(event `/Game/Charlie_EnemyAI_Sandbox/AnimatedInteractables/Interface_Interact.INT_Interact`
  (params (Target :type "Actor Object Reference"))
  (bind _asbp_player_char (cast `/Game/Charlie_EnemyAI_Sandbox/Player/BP_PlayerChar` Target))
  (bind _output_get (set `/Game/Charlie_EnemyAI_Sandbox/Player/BP_PlayerChar.Maxhealth` 200.0 _asbp_player_char))
  (bind _output_get_2 (set `/Game/Charlie_EnemyAI_Sandbox/Player/BP_PlayerChar.Health` 200.0 _asbp_player_char))
  (`/Game/Charlie_EnemyAI_Sandbox/Player/Player_W.SetHealth` (`/Game/Charlie_EnemyAI_Sandbox/Player/BP_PlayerChar.PlayerWidget` _asbp_player_char) _output_get _output_get_2)
  (`self.K2_DestroyActor`))

(fn `UserConstructionScript`)