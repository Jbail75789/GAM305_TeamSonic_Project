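; AI controller for an enemy, labelled as a boss, that runs the AI_BT behavior tree when it possesses a pawn.
; Its AI Perception updates react only to BP_PlayerChar, storing a sensed player as the TargetActor variable and Blackboard key.
; When the player is no longer sensed, both are cleared so the tree sees no target.
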(event `self.ReceivePossess`
  (params (PossessedPawn :type "Pawn Object Reference"))
  ; AI Boss Perception
  (`self.RunBehaviorTree` "/Game/Charlie_EnemyAI_Sandbox/AI/AI_BT.AI_BT"))

(event `self.AIPerception.OnTargetPerceptionUpdated`
  (params (Actor :type "Actor Object Reference") (Stimulus :type "AIStimulus Structure"))
  (bind _returnvalue (`AIBlueprintHelperLibrary.GetBlackboard` self))
  ; AI Boss Perception
  (bind _asbp_player_char (cast `/Game/Charlie_EnemyAI_Sandbox/Player/BP_PlayerChar` Actor))
  (if (`.bSuccessfullySensed` (break `AIStimulus` Stimulus))
    (bind _output_get (set `self.TargetActor` _asbp_player_char))
    (`/Engine/EditorBlueprintResources/StandardMacros.IsValid` _output_get
      (:`Is Valid`
        (`BlackboardComponent.SetValueAsObject` _returnvalue "TargetActor" _output_get)))
    (else
      (bind _output_get_2 (set `self.TargetActor` null))
      (`BlackboardComponent.SetValueAsObject` _returnvalue "TargetActor" _output_get_2))))

(fn `UserConstructionScript`)