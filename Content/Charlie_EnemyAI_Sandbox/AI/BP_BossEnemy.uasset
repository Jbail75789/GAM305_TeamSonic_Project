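; Boss enemy with a health widget, timed projectile fire and player detection.
; The widget yaws toward the player each tick; damage updates it and destroys the boss below zero health.
; Pawn sensing sends one detection message per sighting, using a retriggerable delay to send stop and reset.
; Start/StopShooting toggle the fire timer; the chase branch is empty, FollowPlayer is uncalled, and StopChase issues the move to the player.
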(event `self.ReceiveBeginPlay`
  ; Create Widget on begin play
  (bind _asai_w (cast `/Game/Charlie_EnemyAI_Sandbox/AI/AI_W` (`WidgetComponent.GetUserWidgetObject` (`self.Widget`))))
  (set `self.As AI W` _asai_w))

(event `self.ReceiveTick`
  (params (DeltaSeconds :type "Float (single-precision)"))
  (bind _returnvalue (`GameplayStatics.GetPlayerCharacter` 0))
  (bind _widget (`self.Widget`))
  (bind (_returnvalue_roll _returnvalue_pitch _returnvalue_yaw) (`KismetMathLibrary.BreakRotator` (`KismetMathLibrary.FindLookAtRotation` (`SceneComponent.K2_GetComponentLocation` _widget) (`self.K2_GetActorLocation` _returnvalue))))
  ; get widget location and show players front view
  (`/Engine/EditorBlueprintResources/StandardMacros.IsValid` _returnvalue
    (:`Is Valid`
      (`SceneComponent.K2_SetWorldRotation` _widget (`KismetMathLibrary.MakeRotator` 0.0 0.0 _returnvalue_yaw) false false))))

(event `StartShooting`
  ; Aim at player
  (`KismetSystemLibrary.K2_SetTimer` null "FireatPlayer" (`self.RateofFire`) true))

(event `FollowPlayer`
  ; Aim at player
  (`SceneComponent.K2_SetWorldRotation` (`self.Mesh`) (`KismetMathLibrary.FindLookAtRotation` (`self.K2_GetActorLocation`) (`self.K2_GetActorLocation` (`GameplayStatics.GetPlayerCharacter` (`self.Player Index`)))) false false)
  (`GameplayStatics.PlaySoundAtLocation` "/Engine/VREditor/Sounds/UI/Camera_Shutter.Camera_Shutter" (`self.K2_GetActorLocation`) (struct) 0.1 0.1 0.0 null null null null))

(event `StopShooting`
  ; Aim at player
  (`KismetSystemLibrary.K2_ClearTimer` null "FireatPlayer"))

(event `self.ReceiveAnyDamage`
  (params (Damage :type "Float (single-precision)") (DamageType :type "DamageType Object Reference") (InstigatedBy :type "Controller Object Reference") (DamageCauser :type "Actor Object Reference"))
  ; Damage to player
  (set `self.AIHealth` (- (`self.AIHealth`) Damage))
  (`/Game/Charlie_EnemyAI_Sandbox/AI/AI_W.SetHealth` (`self.As AI W`) (`self.AIHealth`) (`self.AIMaxHealth`))
  (if (< (`self.AIHealth`) 0.0)
    (`self.K2_DestroyActor`)))

(event `FireatPlayer`
  ; Fire at player
  (`|SpawnActorFromClass` "/Game/Charlie_EnemyAI_Sandbox/AI/BP_BossProjectile.BP_BossProjectile_C" (`SceneComponent.K2_GetComponentToWorld` (`self.ProjectileSpawn`)) "Undefined" "MultiplyWithRoot" null null)
  (`KismetSystemLibrary.Delay` 0.4))

(event `self.PawnSensing.OnSeePawn`
  (params (Pawn :type "Pawn Object Reference"))
  ; Start/Stop Detection
  (`|ExecutionSequence`
    (:`then_0`
      (`|ExecutionSequence`
        (:`then_0`
          (`/Engine/EditorBlueprintResources/StandardMacros.DoOnce` false :!label _label
            (:`Completed`
              (message `/Game/Charlie_EnemyAI_Sandbox/Player/DetectionInterface.Start Detection` Pawn self))))
        (:`then_1`
          (if (`self.ShouldChase?`)
            _))))
    (:`then_1`
      (`KismetSystemLibrary.RetriggerableDelay` 0.5)
      (message `/Game/Charlie_EnemyAI_Sandbox/Player/DetectionInterface.StopDetection` Pawn)
      (goto _label :!via `Reset`))))

(event `/Game/Charlie_EnemyAI_Sandbox/Player/DetectionInterface.StartChase`
  ; Start/Stop Detection
  (set `self.ShouldChase?` true))

(event `/Game/Charlie_EnemyAI_Sandbox/Player/DetectionInterface.StopChase`
  ; Start/Stop Detection
  (set `self.ShouldChase?` false)
  (`|AIMoveTo` self (0.0 0.0 0.0) (`GameplayStatics.GetPlayerPawn` 0)))

(fn `UserConstructionScript`)