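; BP_WeaponBase is a base weapon pickup actor that the player can collect.
; Entering or leaving its Sphere shows or hides a Widget component, reacting only to BP_PlayerChar.
; The INTInteract event passes WeaponToSpawn to the interacting BP_PlayerChar's AddWeaponToInventory, then destroys the pickup.
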(event `self.Sphere.OnComponentBeginOverlap`
  (params (OverlappedComponent :type "PrimitiveComponent Object Reference") (OtherActor :type "Actor Object Reference") (OtherComp :type "PrimitiveComponent Object Reference") (OtherBodyIndex :type Integer) (bFromSweep :type Boolean) (SweepResult :type "HitResult Structure (by ref)"))
  (cast `/Game/Charlie_EnemyAI_Sandbox/Player/BP_PlayerChar` OtherActor)
  (`SceneComponent.SetVisibility` (`self.Widget`) true false))

(event `self.Sphere.OnComponentEndOverlap`
  (params (OverlappedComponent :type "PrimitiveComponent Object Reference") (OtherActor :type "Actor Object Reference") (OtherComp :type "PrimitiveComponent Object Reference") (OtherBodyIndex :type Integer))
  (cast `/Game/Charlie_EnemyAI_Sandbox/Player/BP_PlayerChar` OtherActor)
  (`SceneComponent.SetVisibility` (`self.Widget`) false false))

(event `/Game/Charlie_EnemyAI_Sandbox/AnimatedInteractables/Interface_Interact.INT_Interact`
  (params (Target :type "Actor Object Reference"))
  (bind _asbp_player_char (cast `/Game/Charlie_EnemyAI_Sandbox/Player/BP_PlayerChar` Target))
  (`/Game/Charlie_EnemyAI_Sandbox/Player/BP_PlayerChar.AddWeaponToInventory` _asbp_player_char (`self.WeaponToSpawn`))
  (`self.K2_DestroyActor`))

(fn `UserConstructionScript`)