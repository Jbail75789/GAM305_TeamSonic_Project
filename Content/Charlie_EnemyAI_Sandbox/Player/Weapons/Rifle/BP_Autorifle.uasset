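; BP_Autorifle is an interactable rifle actor that gives the player character access to a rifle.
; A sphere overlap shows a widget component when BP_PlayerChar enters and hides it when they leave.
; On interact, it runs the parent's interaction logic, then sets HasRifle on the interacting BP_PlayerChar.
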(event `self.Sphere.OnComponentBeginOverlap`
  (params (OverlappedComponent :type "PrimitiveComponent Object Reference") (OtherActor :type "Actor Object Reference") (OtherComp :type "PrimitiveComponent Object Reference") (OtherBodyIndex :type Integer) (bFromSweep :type Boolean) (SweepResult :type "HitResult Structure (by ref)"))
  (cast `/Game/Charlie_EnemyAI_Sandbox/Player/BP_PlayerChar` OtherActor)
  (`SceneComponent.SetVisibility` (`self.Widget`) true false))

(event `self.Sphere.OnComponentEndOverlap`
  (params (OverlappedComponent :type "PrimitiveComponent Object Reference") (OtherActor :type "Actor Object Reference") (OtherComp :type "PrimitiveComponent Object Reference") (OtherBodyIndex :type Integer))
  (cast `/Game/Charlie_EnemyAI_Sandbox/Player/BP_PlayerChar` OtherActor)
  (`SceneComponent.SetVisibility` (`self.Widget`) false false))

(event `/Game/Charlie_EnemyAI_Sandbox/AnimatedInteractables/Interface_Interact.INT_Interact`
  (params (Target :type "Actor Object Reference"))
  (`parent.INT_Interact` Target)
  (bind _asbp_player_char (cast `/Game/Charlie_EnemyAI_Sandbox/Player/BP_PlayerChar` Target))
  (set `/Game/Charlie_EnemyAI_Sandbox/Player/BP_PlayerChar.HasRifle` true _asbp_player_char))

(fn `UserConstructionScript`
  (`parent.UserConstructionScript`))