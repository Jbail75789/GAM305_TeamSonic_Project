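; BP_PlayerProjectile is a player projectile that damages boss and drone enemies and removes itself after a short lifetime.
; Its Sphere component handles both enemy types: overlaps apply damage to BP_BossEnemy, while blocking hits apply damage to BP_AIDrone.
; Only a drone hit destroys the projectile immediately; it survives boss overlaps and hits on other actors until the BeginPlay delay expires.
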(event `self.ReceiveBeginPlay`
  (`KismetSystemLibrary.Delay` 5.0)
  (`self.K2_DestroyActor`))

(event `self.Sphere.OnComponentBeginOverlap`
  (params (OverlappedComponent :type "PrimitiveComponent Object Reference") (OtherActor :type "Actor Object Reference") (OtherComp :type "PrimitiveComponent Object Reference") (OtherBodyIndex :type Integer) (bFromSweep :type Boolean) (SweepResult :type "HitResult Structure (by ref)"))
  (bind _asbp_boss_enemy (cast `/Game/Charlie_EnemyAI_Sandbox/AI/BP_BossEnemy` OtherActor))
  (`GameplayStatics.ApplyDamage` _asbp_boss_enemy 10.0 null self))

(event `self.Sphere.OnComponentHit`
  (params (HitComponent :type "PrimitiveComponent Object Reference") (OtherActor :type "Actor Object Reference") (OtherComp :type "PrimitiveComponent Object Reference") (NormalImpulse :type "Vector Structure") (Hit :type "HitResult Structure (by ref)"))
  (bind _asbp_aidrone (cast `/Game/BP_AIDrone` OtherActor))
  (`GameplayStatics.ApplyDamage` _asbp_aidrone 10.0 null self)
  (`self.K2_DestroyActor`))

(fn `UserConstructionScript`)