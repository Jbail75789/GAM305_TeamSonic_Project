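; Spider drone enemy built on a parent enemy class, supplying combat range, team and damage handling to the AI.
; Attack fires a targeted MagicSpell through the attacks component from the left shotgun socket, then calls AttackEnd after a fixed delay.
; Damage routes through the damage system component; death plays a montage, enables mesh physics, stops AI logic and hides the health bar.
; AttackStart always succeeds, IsAttacking always returns false, and GetPatrolRoute is empty.
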(event `self.ReceiveBeginPlay`
  (`parent.ReceiveBeginPlay`))

(event `/Game/CameronAI/Task/BPI_EnemyAI_1.Attack`
  (params (AttackTarget :type "Actor Object Reference"))
  (`parent.Attack` AttackTarget)
  (`/Game/CameronAI/Attacks/BPC_Attacks.MagicSpell` (`self.BPC_Attacks1`) (`KismetMathLibrary.MakeTransform` (`SceneComponent.GetSocketLocation` (`self.Mesh`) "ShotgunBot_L")) AttackTarget (make `/Game/CameronAI/DamageSystem/S_DamageInfo_1` 20.0 "NewEnumerator2") false)
  (`KismetSystemLibrary.Delay` 5.0)
  (`self.AttackEnd` AttackTarget))

(event `/Game/CameronAI/Task/BPI_EnemyAI_1.AttackEnd`
  (params (AttackTarget :type "Actor Object Reference")))

(fn `AttackStart`
  (params (AttackTarget :type "Actor Object Reference") (TokensNeeded :type Integer))
  (returns (Success :type Boolean))
  (return true))

(fn `GetIdealRange`
  (returns (AttackRadius :type "Float (double-precision)") (DefendRadius :type "Float (double-precision)"))
  (return 600.0 600.0))

(fn `GetPatrolRoute`
  (returns (PatrolRoute :type "/Game/CameronAI/Enemies/BP_PatrolRoute Object Reference"))
  (return null))

(fn `GetTeamNumber`
  (returns (TeamNumber :type Integer))
  (return (`self.Team Number`)))

(fn `IsAttacking`
  (returns (Attacking :type Boolean))
  (return false))

(fn `OnDeath`
  (bind _mesh (`self.Mesh`))
  (`self.PlayAnimMontage` "/Game/CameronAI/Enemies/SpiderDrone/SpiderDroneDeath.SpiderDroneDeath")
  (`PrimitiveComponent.SetSimulatePhysics` _mesh true)
  (`PrimitiveComponent.SetCollisionEnabled` _mesh "QueryAndPhysics")
  (`BrainComponent.StopLogic` (`AIController.BrainComponent` (`self.AICEnemyBase`)) "")
  (`/Game/CameronAI/Enemies/AIController_BaseEnemy.Set As Dead` (`self.AICEnemyBase`))
  (`SceneComponent.SetVisibility` (`self.HealthBar`) false true))

(fn `TakeDamage`
  (params (DamageInfo :type "/Game/CameronAI/DamageSystem/S_DamageInfo_1 Structure") (`Damage Causer` :type "Actor Object Reference"))
  (returns (WasDamaged :type Boolean))
  (bind _wasdamaged (`/Game/CameronAI/DamageSystem/BPC_DamageSystem.TakeDamage` (`self.BPC_DamageSystem`) DamageInfo `Damage Causer`))
  (return _wasdamaged))

(fn `UserConstructionScript`
  (`parent.UserConstructionScript`))