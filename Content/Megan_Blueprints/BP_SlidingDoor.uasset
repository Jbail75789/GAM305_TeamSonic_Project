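; BP_SlidingDoor is a door that slides along its local Z axis when T is pressed, with input enabled once the player character enters its InteractionZone.
; A FlipFlop alternates each press between playing and reversing the DoorAnimation timeline, whose DoorTrack drives the door's relative location.
; Leaving the zone only casts to the player; DisableInput is unwired, so the door keeps responding to T afterward.
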(event `self.InteractionZone.OnComponentBeginOverlap`
  (params (OverlappedComponent :type "PrimitiveComponent Object Reference") (OtherActor :type "Actor Object Reference") (OtherComp :type "PrimitiveComponent Object Reference") (OtherBodyIndex :type Integer) (bFromSweep :type Boolean) (SweepResult :type "HitResult Structure (by ref)"))
  (cast `/Game/Charlie_EnemyAI_Sandbox/Player/BP_PlayerChar` OtherActor)
  (`self.EnableInput` (`GameplayStatics.GetPlayerController` 0)))

(event `self.InteractionZone.OnComponentEndOverlap`
  (params (OverlappedComponent :type "PrimitiveComponent Object Reference") (OtherActor :type "Actor Object Reference") (OtherComp :type "PrimitiveComponent Object Reference") (OtherBodyIndex :type Integer))
  (cast `/Game/Charlie_EnemyAI_Sandbox/Player/BP_PlayerChar` OtherActor))

(event `Key|T`
  (params (Key :type "Key Structure"))
  (:`Pressed`
    (`/Engine/EditorBlueprintResources/StandardMacros.FlipFlop`
      (:`A`
        (bind (_direction _door_track) (`Timeline|Door Animation` :!label _label)
          (:`Update`
            (`SceneComponent.K2_SetRelativeLocation` (`self.SlidingDoor`) (`KismetMathLibrary.MakeVector` 0.0 0.0 _door_track) false false))))
      (:`B`
        (goto _label :!via `Reverse`)))))

(fn `UserConstructionScript`)