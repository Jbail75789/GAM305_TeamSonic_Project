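; AI drone enemy that detects, aims and fires at the player, with a player-facing health widget and destruction when health drops below zero.
; PawnSensing notifies the seen pawn, using DoOnce and a retriggerable delay to end detection.
; Mesh overlap starts looping timer-driven aiming, while StartFiring and StopFiring events control a projectile-spawning timer.
; Chase is incomplete: FollowPlayer is empty, and StopChase is what issues AIMoveTo toward the player.
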(event `self.ReceiveBeginPlay`
  ; Create Widget on play
  (bind _asai_w (cast `/Game/Charlie_EnemyAI_Sandbox/AI/AI_W` (`WidgetComponent.GetUserWidgetObject` (`self.Widget`))))
  (set `self.AI Widget` _asai_w))

(event `self.ReceiveTick`
  (params (DeltaSeconds :type "Float (single-precision)"))
  (bind _returnvalue (`GameplayStatics.GetPlayerCharacter` 0))
  (bind _widget (`self.Widget`))
  (bind (_returnvalue_roll _returnvalue_pitch _returnvalue_yaw) (`KismetMathLibrary.BreakRotator` (`KismetMathLibrary.FindLookAtRotation` (`SceneComponent.K2_GetComponentLocation` _widget) (`self.K2_GetActorLocation` _returnvalue))))
  ; Show's Widget in players front View
  (`/Engine/EditorBlueprintResources/StandardMacros.IsValid` _returnvalue
    (:`Is Valid`
      (`SceneComponent.K2_SetWorldRotation` _widget (`KismetMathLibrary.MakeRotator` 0.0 0.0 _returnvalue_yaw) false false))))

(event `AimFollowPlayer`
  ; Aim At Player using Pivot
  (`SceneComponent.K2_SetWorldRotation` (`self.Mesh`) (`KismetMathLibrary.FindLookAtRotation` (`self.K2_GetActorLocation`) (`self.K2_GetActorLocation` (`GameplayStatics.GetPlayerCharacter` 0))) false false)
  (`GameplayStatics.PlaySoundAtLocation` "/Engine/VREditor/Sounds/UI/Camera_Shutter.Camera_Shutter" (`self.K2_GetActorLocation`) (struct) 0.1 0.1 0.0 null null null null))

(event `fireAtPlayer`
  ; Fire at player
  (`|SpawnActorFromClass` "/Game/Charlie_EnemyAI_Sandbox/AI/BP_TurretProjectile.BP_TurretProjectile_C" (`SceneComponent.K2_GetComponentToWorld` (`self.ProjectileSpawn`)) "Undefined" "MultiplyWithRoot" null null))

(event `self.Mesh.OnComponentBeginOverlap`
  (params (OverlappedComponent :type "PrimitiveComponent Object Reference") (OtherActor :type "Actor Object Reference") (OtherComp :type "PrimitiveComponent Object Reference") (OtherBodyIndex :type Integer) (bFromSweep :type Boolean) (SweepResult :type "HitResult Structure (by ref)"))
  ; Damage for player
  (`self.AimFollowPlayer`)
  (`KismetSystemLibrary.K2_SetTimer` null "AimFollowPlayer" 0.05 true))

(event `StartFiring`
  ; Damage for player
  (`KismetSystemLibrary.K2_SetTimer` null "fireAtPlayer" (`self.Rateoffire`) true))

(event `self.Mesh.OnComponentEndOverlap`
  (params (OverlappedComponent :type "PrimitiveComponent Object Reference") (OtherActor :type "Actor Object Reference") (OtherComp :type "PrimitiveComponent Object Reference") (OtherBodyIndex :type Integer))
  ; Damage for player
  (`self.FollowPlayer`)
  (`KismetSystemLibrary.K2_ClearTimer` null "AimFollowPlayer"))

(event `StopFiring`
  ; Damage for player
  (`KismetSystemLibrary.K2_ClearTimer` null "fireAtPlayer"))

(event `self.ReceiveAnyDamage`
  (params (Damage :type "Float (single-precision)") (DamageType :type "DamageType Object Reference") (InstigatedBy :type "Controller Object Reference") (DamageCauser :type "Actor Object Reference"))
  ; Damage for player
  (set `self.AIHealth` (- (`self.AIHealth`) Damage))
  (`/Game/Charlie_EnemyAI_Sandbox/AI/AI_W.SetHealth` (`self.AI Widget`) (`self.AIHealth`) (`self.AIMaxHealth`))
  (if (< (`self.AIHealth`) 0.0)
    (`self.K2_DestroyActor`)))

(event `self.PawnSensing.OnSeePawn`
  (params (Pawn :type "Pawn Object Reference"))
  ; Start/Stop Detection
  (`|ExecutionSequence`
    (:`then_0`
      (`|ExecutionSequence`
        (:`then_0`
          (`/Engine/EditorBlueprintResources/StandardMacros.DoOnce` false :!label _label
            (:`Completed`
              (message `/Game/Charlie_EnemyAI_Sandbox/Player/DetectionInterface.StartDetectionTurret` Pawn self))))
        (:`then_1`
          (if (`self.ShouldChase?`)
            (`self.FollowPlayer` self)))))
    (:`then_1`
      (`KismetSystemLibrary.RetriggerableDelay` 0.5)
      (message `/Game/Charlie_EnemyAI_Sandbox/Player/DetectionInterface.StopDetection` Pawn)
      (goto _label :!via `Reset`))))

(event `/Game/Charlie_EnemyAI_Sandbox/Player/DetectionInterface.StartChase`
  ; Start/Stop Detection
  (set `self.ShouldChase?` true))

(event `/Game/Charlie_EnemyAI_Sandbox/Player/DetectionInterface.StopChase`
  ; Start/Stop Detection
  (set `self.ShouldChase?` false)
  (`|AIMoveTo` self (0.0 0.0 0.0) (`GameplayStatics.GetPlayerPawn` 0)))

(fn `FollowPlayer`)

(fn `UserConstructionScript`)