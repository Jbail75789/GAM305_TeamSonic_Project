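; Landmine trap actor that explodes when anything triggers an overlap on its Box component.
; The overlap deals area damage through the BPCAttacks component, spawns a particle effect, plays a sound, fires the ExplosionForce impulse and destroys the actor.
; Health, team, attack-token and damage functions are stubs returning zero or false, so the mine takes no damage.
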(event `self.Box.OnComponentBeginOverlap`
  (params (OverlappedComponent :type "PrimitiveComponent Object Reference") (OtherActor :type "Actor Object Reference") (OtherComp :type "PrimitiveComponent Object Reference") (OtherBodyIndex :type Integer) (bFromSweep :type Boolean) (SweepResult :type "HitResult Structure (by ref)"))
  (bind _returnvalue (`self.K2_GetActorLocation`))
  (`/Game/CameronAI/Attacks/BPC_Attacks.AOEDamage` (`self.BPC_Attacks`) 500.0 (make `/Game/CameronAI/DamageSystem/S_DamageInfo_1` 20.0))
  (`GameplayStatics.SpawnEmitterAtLocation` "/Engine/Tutorial/SubEditors/TutorialAssets/TutorialParticleSystem.TutorialParticleSystem" _returnvalue)
  (`GameplayStatics.PlaySoundAtLocation` null _returnvalue (struct) 1.0 1.0 0.0 null null null null)
  (`RadialForceComponent.FireImpulse` (`self.ExplosionForce`))
  (`self.K2_DestroyActor`))

(fn `GetCurrentHealth`
  (returns (Health :type "Float (double-precision)"))
  (return 0.0))

(fn `GetMaxHealth`
  (returns (MaxHealth :type "Float (double-precision)"))
  (return 0.0))

(fn `GetTeamNumber`
  (returns (TeamNumber :type Integer))
  (return 0))

(fn `Heal`
  (params (Amount :type "Float (double-precision)"))
  (returns (NewHealth :type "Float (double-precision)"))
  (return 0.0))

(fn `IsAttacking`
  (returns (Attacking :type Boolean))
  (return false))

(fn `IsDead`
  (returns (Dead :type Boolean))
  (return false))

(fn `ReserveAttackToken`
  (params (Amount :type Integer))
  (returns (Success :type Boolean))
  (return false))

(fn `TakeDamage`
  (params (DamageInfo :type "/Game/CameronAI/DamageSystem/S_DamageInfo_1 Structure") (`Damage Causer` :type "Actor Object Reference"))
  (returns (WasDamaged :type Boolean))
  (return false))

(fn `UserConstructionScript`)