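; Explosive barrel actor that detonates when accumulated damage depletes its health.
; Any damage lowers Health, and at zero or below a DoOnce gate triggers the explosion a single time.
; The explosion applies radial damage, spawns a particle effect, plays a sound and fires the ExplosionForce impulse before the actor destroys itself.
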(event `self.ReceiveAnyDamage`
  (params (Damage :type "Float (single-precision)") (DamageType :type "DamageType Object Reference") (InstigatedBy :type "Controller Object Reference") (DamageCauser :type "Actor Object Reference"))
  (bind _returnvalue (`self.K2_GetActorLocation`))
  (bind _output_get (set `self.Health` (- (`self.Health`) Damage)))
  (if (<= _output_get 0.0)
    (`/Engine/EditorBlueprintResources/StandardMacros.DoOnce` false
      (:`Completed`
        (`GameplayStatics.ApplyRadialDamage` :`BaseDamage` 100.0 :`Origin` _returnvalue :`DamageRadius` 500.0 :`DamageCauser` null :`InstigatedByController` null)
        (`GameplayStatics.SpawnEmitterAtLocation` "/Engine/Tutorial/SubEditors/TutorialAssets/TutorialParticleSystem.TutorialParticleSystem" _returnvalue)
        (`GameplayStatics.PlaySoundAtLocation` null _returnvalue (struct) 1.0 1.0 0.0 null null null null)
        (`RadialForceComponent.FireImpulse` (`self.ExplosionForce`))
        (`self.K2_DestroyActor`)))))

(fn `UserConstructionScript`)